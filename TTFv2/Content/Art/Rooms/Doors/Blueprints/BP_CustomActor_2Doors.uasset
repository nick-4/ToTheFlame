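; Double door actor that swings open when the main character, a human or a mutant enters its trigger box, and closes when one leaves.
; A timeline drives mirrored yaw on four scene components up to a maximum angle, reversing to close and updating IsOpen on finish.
; The construction script applies the initial open pose and sizes and raises the box.
; DoorInProgress is only ever set false, so its guard never blocks.
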(event `self.ReceiveBeginPlay`
  (`parent.ReceiveBeginPlay`)
  (set `PrimitiveComponent.bGenerateOverlapEvents` (`self.EnableOverlap`) (`self.Box`)))

(event `self.Box.OnComponentBeginOverlap`
  (params (OverlappedComponent :type "PrimitiveComponent Object Reference") (OtherActor :type "Actor Object Reference") (OtherComp :type "PrimitiveComponent Object Reference") (OtherBodyIndex :type Integer) (bFromSweep :type Boolean) (SweepResult :type "HitResult Structure (by ref)"))
  (`|ExecutionSequence`
    (:`then_0`
      (cast `/Game/TTF/Blueprints/Characters/BP_TTF_MainCharacter` OtherActor))
    (:`then_1`
      (cast `/Game/TTF/Blueprints/Characters/Enemies/BP_BaseHuman` OtherActor))
    (:`then_2`
      (cast `/Game/TTF/Blueprints/Characters/Enemies/BP_BaseMutant` OtherActor)))
  (`self.DoorOpen`))

(event `self.Box.OnComponentEndOverlap`
  (params (OverlappedComponent :type "PrimitiveComponent Object Reference") (OtherActor :type "Actor Object Reference") (OtherComp :type "PrimitiveComponent Object Reference") (OtherBodyIndex :type Integer))
  (`|ExecutionSequence`
    (:`then_0`
      (cast `/Game/TTF/Blueprints/Characters/BP_TTF_MainCharacter` OtherActor))
    (:`then_1`
      (cast `/Game/TTF/Blueprints/Characters/Enemies/BP_BaseHuman` OtherActor))
    (:`then_2`
      (cast `/Game/TTF/Blueprints/Characters/Enemies/BP_BaseMutant` OtherActor)))
  (`self.DoorClose`))

(event `DoorOpen`
  (if (not (`self.DoorInProgress`))
    (if (not (`self.IsOpen`))
      (bind (_direction _dooropenprogression) (`Timeline|Timeline_0` :!via `PlayFromStart` :!label _label)
        (:`Update`
          (set `self.DoorInProgress` false)
          (bind _returnvalue (* _dooropenprogression (`self.MaxDoorOpenAngle`)))
          (`SceneComponent.K2_SetRelativeRotation` (`self.SceneLeft`) (`KismetMathLibrary.MakeRotator` 0.0 0.0 _returnvalue) false false)
          (bind _returnvalue_2 (* _returnvalue -1.0))
          (`SceneComponent.K2_SetRelativeRotation` (`self.SceneRight`) (`KismetMathLibrary.MakeRotator` 0.0 0.0 _returnvalue_2) false false)
          (`SceneComponent.K2_SetRelativeRotation` (`self.SceneDoorLeft`) (`KismetMathLibrary.MakeRotator` 0.0 0.0 _returnvalue_2) false false)
          (`SceneComponent.K2_SetRelativeRotation` (`self.SceneDoorRight`) (`KismetMathLibrary.MakeRotator` 0.0 0.0 _returnvalue) false false))
        (:`Finished`
          (set `self.DoorInProgress` false)
          (switch `ETimelineDirection` _direction
            (:`Forward`
              (set `self.IsOpen` true))
            (:`Backward`
              (set `self.IsOpen` false))))))))

(event `DoorClose`
  (if (not (`self.DoorInProgress`))
    (if (`self.IsOpen`)
      (goto _label :!via `Reverse`))))

(fn `UserConstructionScript`
  (`parent.UserConstructionScript`)
  (`|ExecutionSequence`
    (:`then_0`
      (`SceneComponent.K2_AddRelativeRotation` (`self.SceneLeft`) (`KismetMathLibrary.MakeRotator` 0.0 0.0 (select `bool` (`self.IsOpen`) :`true` (`self.MaxDoorOpenAngle`))) false false)
      (`SceneComponent.K2_AddRelativeRotation` (`self.SceneRight`) (`KismetMathLibrary.MakeRotator` 0.0 0.0 (select `bool` (`self.IsOpen`) :`true` (* (`self.MaxDoorOpenAngle`) -1.0))) false false)
      (`SceneComponent.K2_AddRelativeRotation` (`self.SceneDoorLeft`) (`KismetMathLibrary.MakeRotator` 0.0 0.0 (select `bool` (`self.IsOpen`) :`true` (* (`self.MaxDoorOpenAngle`) -1.0))) false false)
      (`SceneComponent.K2_AddRelativeRotation` (`self.SceneDoorRight`) (`KismetMathLibrary.MakeRotator` 0.0 0.0 (select `bool` (`self.IsOpen`) :`true` (`self.MaxDoorOpenAngle`))) false false))
    (:`then_1`
      (`BoxComponent.SetBoxExtent` (`self.Box`) (`self.BoxExtent`) true)
      (`SceneComponent.K2_AddRelativeLocation` (`self.Box`) (`KismetMathLibrary.MakeVector` 0.0 0.0 (.z (`self.BoxExtent`))) false false))))