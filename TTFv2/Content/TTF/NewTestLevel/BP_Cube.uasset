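; BP_Cube is an actor whose cube spins continuously and moves vertically, driven by per-instance speed variables.
; BeginPlay sets the RotatingMovement component's rate and the CubeUPDown timeline's play rate, then plays the timeline through its component reference.
; The timeline's update output lerps the cube's relative Z between fixed lower and upper offsets.
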(event `self.ReceiveBeginPlay`
  (`TimelineComponent.SetPlayRate` (`self.CubeUPDown`) (`self.CubCycleUpDown`))
  (set `RotatingMovementComponent.RotationRate` (`KismetMathLibrary.MakeRotator` 0.0 0.0 (`self.CubRotationSpeed`)) (`self.RotatingMovement`))
  (`TimelineComponent.Play` (`self.CubeUPDown`)))

(fn `UserConstructionScript`)