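; Deprecated copy of a light bar actor that finds light-vulnerable actors in its beam through line traces.
; TraceForTargets fires a square grid of debug-drawn Pawn-profile traces along world +X from the actor's location, ignoring its rotation.
; Hit actors implementing BPI_LightVulnerable are deduplicated through a set and returned as interface references.
; The event graph is empty, and a channel-trace variant is left unconnected.
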(fn `TraceForTargets`
  (returns (Targets :type "Array of /Game/TTF/Blueprints/Lights/BPI_LightVulnerable Interface"))
  (for _index (range -3 4)
    (for _index_2 (range -3 4)
      (bind _returnvalue (+ (`KismetMathLibrary.MakeVector` 0.0 (* _index 16.0) (* _index_2 16.0)) (`self.K2_GetActorLocation`)))
      (bind _outhit (`KismetSystemLibrary.LineTraceSingleByProfile` :`Start` _returnvalue :`End` (+ _returnvalue (4000.0 0.0 0.0)) :`ProfileName` "Pawn" :`DrawDebugType` "ForOneFrame"))
      (cast `/Game/TTF/Blueprints/Lights/BPI_LightVulnerable` (`.HitActor` (`GameplayStatics.BreakHitResult` _outhit)))
      (`BlueprintSetLibrary.Set_Add` (`self.TraceResults`) (`.HitActor` (`GameplayStatics.BreakHitResult` _outhit)))))
  (bind _result (`BlueprintSetLibrary.Set_ToArray` (`self.TraceResults`)))
  (for _array_element _result
    (bind _asbpi_light_vulnerable (cast `/Game/TTF/Blueprints/Lights/BPI_LightVulnerable` _array_element))
    (`KismetArrayLibrary.Array_Add` (`self.TraceResultsInterfaced`) _asbpi_light_vulnerable))
  (return (`self.TraceResultsInterfaced`)))

(fn `UserConstructionScript`
  (`parent.UserConstructionScript`))