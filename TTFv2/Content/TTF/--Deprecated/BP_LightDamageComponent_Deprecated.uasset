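; Deprecated light damage component that relays damage and danger notifications to actors implementing BPI_LightVulnerable.
; Danger events call StartDanger and EndDanger on the target through the interface.
; StartDamaging makes one CauseLightDamage call with zero damage, leaving DamagePerSecond unused.
; StopDamaging only performs the cast, and the StartDangerSignal and StopDangerSignal graphs are empty.
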(event `Start Damaging`
  (params (Actor :type "Actor Object Reference"))
  ;[1 1 1] Damage
  (`self.StartDamaging` Actor))

(event `Stop Damaging`
  (params (Actor :type "Actor Object Reference"))
  ;[1 1 1] Damage
  (`self.StopDamaging` Actor))

(event `Notify Danger`
  (params (Actor :type "Actor Object Reference"))
  ;[1 1 1] Danger
  (bind _asbpi_light_vulnerable (cast `/Game/TTF/Blueprints/Lights/BPI_LightVulnerable` Actor))
  (`/Game/TTF/Blueprints/Lights/BPI_LightVulnerable.StartDanger` _asbpi_light_vulnerable))

(event `Notify Danger End`
  (params (Actor :type "Actor Object Reference"))
  ;[1 1 1] Danger
  (bind _asbpi_light_vulnerable (cast `/Game/TTF/Blueprints/Lights/BPI_LightVulnerable` Actor))
  (`/Game/TTF/Blueprints/Lights/BPI_LightVulnerable.EndDanger` _asbpi_light_vulnerable))