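; BP_DashInactive is an actor that switches the player to a no-dash controller as soon as it begins play.
; BeginPlay prints a debug string, unpossesses the TopDownController, then spawns a TopDownControllerNoDash at the character mesh's transform to possess the same character.
; The Box overlap event is empty, and the disconnected logic that shows a main UI image never runs.
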(event `self.ReceiveBeginPlay`
  (bind _returnvalue (`GameplayStatics.GetPlayerCharacter` 0))
  (`KismetSystemLibrary.PrintString` "Hello" true true (struct :`R` 0.90809 :`G` 0.016356 :`B` 1.0 :`A` 1.0))
  (bind _astop_down_controller (cast `/Game/TopDownBP/Blueprints/TopDownController` (`GameplayStatics.GetPlayerController` 0)))
  (`Controller.UnPossess` _astop_down_controller)
  (bind _returnvalue_2 (`|SpawnActorFromClass` "/Game/TopDownBP/Blueprints/TopDownControllerNoDash.TopDownControllerNoDash_C" (`SceneComponent.K2_GetComponentToWorld` (`Character.Mesh` _returnvalue)) "Undefined" "OverrideRootScale" _returnvalue null))
  (bind _output_get (set `self.NewVar_2` _returnvalue_2))
  (`Controller.Possess` _output_get _returnvalue))

(event `self.Box.OnComponentBeginOverlap`
  (params (OverlappedComponent :type "PrimitiveComponent Object Reference") (OtherActor :type "Actor Object Reference") (OtherComp :type "PrimitiveComponent Object Reference") (OtherBodyIndex :type Integer) (bFromSweep :type Boolean) (SweepResult :type "HitResult Structure (by ref)")))

(fn `UserConstructionScript`)