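; BP_TTFCharacterTest is a test character Blueprint that creates the main game UI and provides a placeholder danger signal.
; BeginPlay creates a GameMainUI widget, stores it and adds it to the viewport.
; StartDanger fires DangerTick immediately, then repeats it on a looping timer that prints a red debug message until EndDanger clears it.
; The UpdateHealthBar override only calls its parent implementation.
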(event `self.ReceiveBeginPlay`
  ;[1 1 1] Initialise
  (bind _returnvalue (`|CreateWidget` "/Game/TTF/Blueprints/GameMainUI.GameMainUI_C"))
  (bind _output_get (set `self.GameMainUIW` _returnvalue))
  (`UserWidget.AddToViewport` _output_get 0))

(event `/Game/TTF/Blueprints/Lights/BPI_LightVulnerable.EndDanger`
  ;[1 1 1] Danger Signal
  (`KismetSystemLibrary.K2_ClearAndInvalidateTimerHandle` (`self.DangerSignalTimer`)))

(event `/Game/TTF/Blueprints/Lights/BPI_LightVulnerable.StartDanger`
  ;[1 1 1] Danger Signal
  (`self.Danger Tick`)
  (bind _returnvalue (`KismetSystemLibrary.K2_SetTimerDelegate` (delegate `Danger Tick`) 1.0 true))
  (set `self.DangerSignalTimer` _returnvalue))

(event `Danger Tick`
  ;[1 1 1] Danger Signal
  ;;[1 1 1] Danger Tick
  (`KismetSystemLibrary.PrintString` "Danger" true true (struct :`R` 1.0 :`B` 0.126089 :`A` 1.0) 0.5))

(fn `UpdateHealthBar`
  (`parent.UpdateHealthBar`))

(fn `UserConstructionScript`)