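; Base character Blueprint for TTF that manages health and ragdoll death.
; Construction sets Health to StartHealth, and ChangeHealth applies signed changes clamped between zero and MaxHealth.
; The Health RepNotify calls an empty health bar update hook, fires the OnHealthUpdated dispatcher and checks for death.
; At zero health, a one-time ragdoll switch disables movement and capsule collision, then enables physics simulation on the mesh.
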(fn `ChangeHealth`
  (params (ChangeValue :type "Float (double-precision)"))
  (set `self.Health` (`KismetMathLibrary.FClamp` (+ ChangeValue (`self.Health`)) 0.0 (`self.MaxHealth`))))

(fn `OnRep_Health`
  (`self.UpdateHealthBarMethod`)
  (`self.OnHealthUpdated` (`self.Health`) (`self.MaxHealth`))
  (`self.TurnOnRagdollIfNeeded`))

(fn `UpdateHealthBarMethod`)

(fn `UserConstructionScript`
  (`self.Initialize`)
  (`KismetSystemLibrary.PrintString` "Constructor"))