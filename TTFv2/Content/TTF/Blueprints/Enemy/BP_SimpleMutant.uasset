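; Enemy Blueprint for a simple mutant, with a widget health bar and AI perception.
; It sets the bar from Health over MaxHealth on BeginPlay and after the parent's health bar update method.
; AnyDamage passes damage to TakeDamage, though the local TakeDamage macro graph holds only unconnected leftover logic.
; Perception updates are rebroadcast through the TargetPerceptionUpdated dispatcher.
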(event `self.ReceiveBeginPlay`
  (`self.SetHealthBarValue`))

(event `self.ReceiveAnyDamage`
  (params (Damage :type "Float (single-precision)") (DamageType :type "DamageType Object Reference") (InstigatedBy :type "Controller Object Reference") (DamageCauser :type "Actor Object Reference"))
  ;[1 1 1] Take Damage ??????????????
  (`self.TakeDamage` Damage))

(event `self.AIPerception.OnTargetPerceptionUpdated`
  (params (Actor :type "Actor Object Reference") (Stimulus :type "AIStimulus Structure"))
  ;[1 1 1] Dispatch Perception Event
  (`self.TargetPerceptionUpdated` Actor Stimulus))

(fn `UpdateHealthBarMethod`
  (`parent.UpdateHealthBarMethod`)
  (`self.SetHealthBarValue`))

(fn `UserConstructionScript`
  (`parent.UserConstructionScript`))