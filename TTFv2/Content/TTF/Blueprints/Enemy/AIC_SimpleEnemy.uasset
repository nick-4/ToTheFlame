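; AI controller for the simple mutant enemy that runs its behavior tree on possess and feeds perception results into the Blackboard.
; On BeginPlay it binds to the possessed BP_SimpleMutant's target perception updates, setting the line-of-sight key and target actor on each sighting.
; Losing sight starts a short grace timer that clears the target actor on expiry; a new successful sensing cancels it.
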(event `self.ReceivePossess`
  (params (PossessedPawn :type "Pawn Object Reference"))
  ;[1 1 1] On Possess Run Behavior Tree
  (`self.RunBehaviorTree` "/Game/TTF/Blueprints/Enemy/AI/BT_SimpleEnemyAI.BT_SimpleEnemyAI"))

(event `self.ReceiveBeginPlay`
  ;[1 1 1] Begin Play - Subscribe Perception Event
  (bind _asbp_simple_mutant (cast `/Game/TTF/Blueprints/Enemy/BP_SimpleMutant` (`self.K2_GetPawn`)))
  (add `/Game/TTF/Blueprints/Enemy/BP_SimpleMutant.TargetPerceptionUpdated` _asbp_simple_mutant (delegate `HandleTargetPerceptionUpdated`)))

(event `HandleTargetPerceptionUpdated`
  (params (PerceivedActor :type "Actor Object Reference") (Stimulus :type "AIStimulus Structure"))
  (bind ((`StimulusLocation` _stimuluslocation) (`bSuccessfullySensed` _bsuccessfullysensed)) (break `AIStimulus` Stimulus))
  ;[1 1 1] Update Blackboard Data
  (`self.UpdateHasLineOfSightKey` _bsuccessfullysensed)
  (if _bsuccessfullysensed
    (`KismetSystemLibrary.K2_ClearAndInvalidateTimerHandle` (`self.Target Lost Timer`))
    (`self.UpdateTargetActorKey` PerceivedActor)
    (else
      (bind _returnvalue (`KismetSystemLibrary.K2_SetTimerDelegate` (delegate `TargetIsLost`) 2.0))
      (set `self.Target Lost Timer` _returnvalue))))

(event `TargetIsLost`
  ;[1 1 1] Target Is Lost
  (`self.UpdateTargetActorKey` null))

(fn `UpdateHasLineOfSightKey`
  (params (BoolValue :type Boolean))
  (`BlackboardComponent.SetValueAsBool` (`self.Blackboard`) (`self.HasLineOfSightName`) BoolValue))

(fn `UpdateTargetActorKey`
  (params (ObjectValue :type "Object Object Reference"))
  (`BlackboardComponent.SetValueAsObject` (`self.Blackboard`) (`self.TargetActorName`) ObjectValue))

(fn `UserConstructionScript`)