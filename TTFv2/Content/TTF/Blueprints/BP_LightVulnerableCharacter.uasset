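; Character Blueprint for taking damage over time from light, currently a stub that prints the damage without reducing any health.
; A looping timer started on BeginPlay passes the current damage rate times the tick period to ApplyLightDamage.
; RemoveLightDamage_1 lowers the rate, while CauseLightDamage adds only zero to it.
; ApplyLightDamage prints positive amounts and calls UpdateHealthBar, which is empty.
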(event `self.ReceiveBeginPlay`
  ;[0 1 0.05297] Initialize
  (`self.Start Light Damage Timer`))

(event `Apply Light Damage`
  (params (`Damage Value` :type "Float (double-precision)"))
  ;[1 0.2448 0.2448] Damage
  ;;[1 0.704 0.6641] Apply Damage
  (`self.ApplyLightDamage` `Damage Value`))

(event `/Game/TTF/Blueprints/Lights/BPI_LightVulnerable2.CauseLightDamage`
  (params (Damage :type "Float (single-precision)"))
  ;[1 0.2448 0.2448] Damage
  ;;[1 0.625 0.625] Change Light Damage
  (set `self.CurrentLightDamageSpeed` (+ 0.0 (`self.CurrentLightDamageSpeed`))))

(event `Start Light Damage Timer`
  ;[1 0.2448 0.2448] Damage
  ;;[1 0.7171 0.6972] Damage Timer
  (`KismetSystemLibrary.K2_SetTimerDelegate` (delegate `LightDamage Tick`) (`self.ApplyDamagePeriod`) true))

(event `RemoveLightDamage_1`
  (params (DamagePerSecond :type "Float (double-precision)"))
  ;[1 0.2448 0.2448] Damage
  ;;[1 0.625 0.625] Change Light Damage
  (set `self.CurrentLightDamageSpeed` (- (`self.CurrentLightDamageSpeed`) DamagePerSecond)))

(event `LightDamage Tick`
  ;[1 0.2448 0.2448] Damage
  ;;[1 0.7171 0.6972] Damage Timer
  (`self.Apply Light Damage` (* (`self.ApplyDamagePeriod`) (`self.CurrentLightDamageSpeed`))))

(fn `UpdateHealthBar`)

(fn `UserConstructionScript`
  (`parent.UserConstructionScript`))