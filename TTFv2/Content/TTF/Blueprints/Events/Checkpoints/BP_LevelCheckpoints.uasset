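; BP_LevelCheckpoints restores the main character to the last saved checkpoint when a level begins.
; On BeginPlay it loads the "Autosave" save and looks up the saved checkpoint ID in CheckpointsDict.
; A valid match teleports MainCharacter to that checkpoint's location.
; It also enables player input so the R key can print a debug string and call StartClearGame.
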(event `self.ReceiveBeginPlay`
  (`self.Enable User Input`)
  (bind _waypoint (`self.If Have Valid Save`)
    (:`Is Valid`
      (`self.MoveMainCharacterToCheckpoint` _waypoint))))

(event `Key|R`
  (params (Key :type "Key Structure"))
  (:`Pressed`
    (`KismetSystemLibrary.PrintString` "RRRRRRRRRRRRRRRRRR")
    (`/Game/TTF/Blueprints/BPFL_Helpers.StartClearGame`)))

(fn `Enable User Input`
  (`self.EnableInput` (`GameplayStatics.GetPlayerController` 0)))

(fn `UserConstructionScript`)