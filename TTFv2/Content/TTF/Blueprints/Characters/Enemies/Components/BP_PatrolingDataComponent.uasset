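; Patrol data component for enemy characters that picks the next location to move to while patrolling.
; ChooseNextLocation returns the location of a waypoint actor, either the next in looping order or a random one, depending on RandomizeWaypoints.
; Random selection re-rolls until the index differs from the current one when multiple waypoints exist.
; With no waypoints, it falls back to a random reachable navigation point within a radius of the owner.
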(fn `ChooseNextLocation`
  (returns (Location :type "Vector Structure"))
  (if (== (`KismetArrayLibrary.Array_Length` (`self.Waypoints`)) 0)
    (bind _location (`self.GetRandomReachableLocation`))
    (return _location)
    (elif (`self.RandomizeWaypoints?`)
      (bind _actor (`self.GetRandomWaypoint`))
      (return (`Actor.K2_GetActorLocation` _actor))
      (else
        (bind _actor_2 (`self.GetNextWaypoint`))
        (return (`Actor.K2_GetActorLocation` _actor_2))))))

(fn `GetNextWaypoint`
  (returns (Actor :type "Actor Object Reference"))
  (bind _result (`/Engine/EditorBlueprintResources/StandardMacros.IncrementInt` (`self.CurrentIndex`))
    (:`  `
      (bind _output_get (set `self.CurrentIndex` (mod _result (`KismetArrayLibrary.Array_Length` (`self.Waypoints`)))))
      (return (`|GetArrayItem` (`self.Waypoints`) _output_get)))))

(fn `GetRandomReachableLocation`
  (returns (Location :type "Vector Structure"))
  (return (`NavigationSystemV1.K2_GetRandomReachablePointInRadius` (`Actor.K2_GetActorLocation` (`self.GetOwner`)) (`self.RandomLocationRadius`) null null)))

(fn `GetRandomWaypoint`
  (returns (Actor :type "Actor Object Reference"))
  (locals (index :type Integer) (max :type Integer))
  (`|ExecutionSequence`
    (:`then_0`
      ;[1 1 1] Set local variables
      (set `local.max` (`KismetArrayLibrary.Array_Length` (`self.Waypoints`)))
      (set `local.index` (`self.CurrentIndex`)))
    (:`then_1`
      ;[1 1 1] If at least 2 elements
      (if (> (`local.max`) 1)
        ;[1 1 1] Find Random Index
        (while (== (`local.index`) (`self.CurrentIndex`))
          (set `local.index` (`KismetMathLibrary.RandomInteger` (`local.max`))))
        (set `self.CurrentIndex` (`local.index`))))
    (:`then_2`
      ;[1 1 1] Return waypoint by index
      (return (`|GetArrayItem` (`self.Waypoints`) (`local.index`))))))