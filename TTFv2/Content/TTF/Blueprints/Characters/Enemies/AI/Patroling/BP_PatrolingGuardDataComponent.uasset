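; Data component for patrolling guard AI that supplies the next patrol location and identifies which actors count as enemies.
; ChooseNextLocation returns a waypoint actor's location, picked either randomly or in looping order according to RandomizeWaypoints.
; Random picks re-roll until the index differs from the current one, so a single-waypoint list would loop endlessly.
; Enemy checks match an actor's exact class against EnemyClasses, so unlisted subclasses do not count.
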(fn `ChooseNextLocation`
  (returns (Location :type "Vector Structure"))
  (if (`self.RandomizeWaypoints?`)
    (bind _actor (`self.GetRandomWaypoint`))
    (return (`Actor.K2_GetActorLocation` _actor))
    (else
      (bind _actor_2 (`self.GetNextWaypoint`))
      (return (`Actor.K2_GetActorLocation` _actor_2)))))

(fn `GetNextWaypoint`
  (returns (Actor :type "Actor Object Reference"))
  (bind _result (`/Engine/EditorBlueprintResources/StandardMacros.IncrementInt` (`self.CurrentIndex`))
    (:`  `
      (bind _output_get (set `self.CurrentIndex` (mod _result (`KismetArrayLibrary.Array_Length` (`self.Waypoints`)))))
      (return (`|GetArrayItem` (`self.Waypoints`) _output_get)))))

(fn `GetRandomWaypoint`
  (returns (Actor :type "Actor Object Reference"))
  (locals (index :type Integer) (max :type Integer))
  (set `local.max` (`KismetArrayLibrary.Array_Length` (`self.Waypoints`)))
  (set `local.index` (`self.CurrentIndex`))
  (while (== (`local.index`) (`self.CurrentIndex`))
    (set `local.index` (`KismetMathLibrary.RandomInteger` (`local.max`))))
  (bind _output_get (set `self.CurrentIndex` (`local.index`)))
  (return (`|GetArrayItem` (`self.Waypoints`) _output_get)))

(fn `IsEnemy`
  (params (Actor :type "Actor Object Reference"))
  (returns (Yes :type Boolean))
  (return (`self.IsEnemyClass` (`GameplayStatics.GetObjectClass` Actor))))

(fn `IsEnemyClass`
  (params (ClassToTest :type "Actor Class Reference"))
  (returns (IsInList :type Boolean))
  (return (`KismetArrayLibrary.Array_Contains` (`self.EnemyClasses`) ClassToTest)))