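; BP_BaseChar is a base character with health, melee damage intake, stone throwing and ragdoll death.
; Health starts at StartHealth and changes through a clamped setter, with its RepNotify refreshing the overhead widget bar, calling OnHealthUpdated and checking for death.
; Death disables movement and capsule collision, enables mesh physics and hides the health bar.
; Throwing spawns BP_Stone from a mesh socket, angled from the forward vector by ThrowVerticalAngle.
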(event `self.ReceiveBeginPlay`
  (`self.UpdateHealthBar`))

(fn `ApplyMeleeDamage`
  (params (Amount :type "Float (double-precision)"))
  (bind _result (`/Engine/EditorBlueprintResources/StandardMacros.NegateFloat` Amount)
    (:`  `
      (`self.ChangeHealth` _result))))

(fn `ChangeHealth`
  (params (ChangeValue :type "Float (double-precision)"))
  (set `self.Health` (`KismetMathLibrary.FClamp` (+ ChangeValue (`self.Health`)) 0.0 (`self.MaxHealth`))))

(fn `Die`
  (set `self.IsDead?` true)
  (`self.RagdollOn`)
  (`self.TurnPersonalHealthBarOn` false))

(fn `OnRep_Health`
  (`self.UpdateHealthBar`)
  (`self.OnHealthUpdated` (`self.Health`) (`self.MaxHealth`))
  (`self.CheckHealthAndDieIfNeeded`))

(fn `Throw`
  (`self.ThrowProjectile` (`SceneComponent.GetSocketLocation` (`self.Mesh`) (`self.TrowingSlotName`)) (`KismetMathLibrary.RotateAngleAxis` (`self.GetActorForwardVector`) (- 0.0 (`self.ThrowVerticalAngle`)) (`self.GetActorRightVector`)) "/Game/TTF/Blueprints/Objects/BP_Stone.BP_Stone_C"))

(fn `ThrowProjectile`
  (params (StartPosition :type "Vector Structure") (Direction :type "Vector Structure") (ProjectileClass :type "Actor Class Reference"))
  (`|SpawnActorFromClass` ProjectileClass (`KismetMathLibrary.MakeTransform` StartPosition (`KismetMathLibrary.MakeRotFromX` Direction)) "AlwaysSpawn" "OverrideRootScale" null self))

(fn `TurnPersonalHealthBarOn`
  (params (bNewVisibility :type Boolean))
  (`SceneComponent.SetVisibility` (`self.HealthBarWidget`) bNewVisibility true))

(fn `UpdateHealthBar`
  (bind _aswbp_personal_health_bar (cast `/Game/TTF/Blueprints/Widgets/WBP_PersonalHealthBar` (`WidgetComponent.GetUserWidgetObject` (`self.HealthBarWidget`))))
  (`ProgressBar.SetPercent` (`/Game/TTF/Blueprints/Widgets/WBP_PersonalHealthBar.HealthProgressBar` _aswbp_personal_health_bar) (/ (`self.Health`) (`self.MaxHealth`))))

(fn `UserConstructionScript`
  (`self.Initialize`))