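; Character Blueprint for characters that lose health when exposed to light.
; CauseLightDamage passes incoming damage to GetLightDamage, which converts it into a ChangeHealth call.
; A periodic damage-over-time path, marked deprecated, remains: a looping timer applies the current damage speed scaled by the period, but its start call is disconnected.
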(event `self.ReceiveBeginPlay`
  ;[0 1 0.05297] Initialize
  (`parent.ReceiveBeginPlay`))

(event `/Game/TTF/Blueprints/Lights/BPI_LightVulnerableV2.CauseLightDamage`
  (params (Damage :type "Float (single-precision)"))
  ;[1 0.2448 0.2448] Damage
  (`self.GetLightDamage` Damage))

(event `Start Light Damage Timer`
  ;[0.08738 0 0.2448] Deprecated
  ;;[1 0.7171 0.6972] Damage Timer
  (`KismetSystemLibrary.K2_SetTimerDelegate` (delegate `LightDamage Tick`) (`self.ApplyDamagePeriod`) true))

(event `RemoveLightDamage_1`
  (params (DamagePerSecond :type "Float (double-precision)"))
  ;[0.08738 0 0.2448] Deprecated
  ;;[1 0.625 0.625] Change Light Damage
  (set `self.CurrentLightDamageSpeed` (- (`self.CurrentLightDamageSpeed`) DamagePerSecond)))

(event `LightDamage Tick`
  ;[0.08738 0 0.2448] Deprecated
  ;;[1 0.7171 0.6972] Damage Timer
  (`self.Apply Light Damage` (* (`self.ApplyDamagePeriod`) (`self.CurrentLightDamageSpeed`))))

(event `Apply Light Damage`
  (params (`Damage Value` :type "Float (double-precision)"))
  ;[0.08738 0 0.2448] Deprecated
  ;;[1 0.704 0.6641] Apply Damage
  (`self.GetLightDamage` `Damage Value`))

(fn `UserConstructionScript`
  (`parent.UserConstructionScript`))