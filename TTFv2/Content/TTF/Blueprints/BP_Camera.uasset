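; Camera actor for a top-down game that detects what sits between its Camera2 component and the player's pawn.
; Each tick it runs a debug-drawn capsule trace on the Visibility channel toward the pawn and prints the hit actor's name.
; BeginPlay sets the TopDownController's PlayerCamera to None.
; A material swap to M_LocationOpacity is present but unwired, so occluders are only reported, never altered.
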(event `self.ReceiveBeginPlay`
  (bind _astop_down_controller (cast `/Game/TopDownBP/Blueprints/TopDownController` (`GameplayStatics.GetPlayerController` 0)))
  (set `/Game/TopDownBP/Blueprints/TopDownController.PlayerCamera` null _astop_down_controller))

(event `self.ReceiveTick`
  (params (DeltaSeconds :type "Float (single-precision)"))
  (bind _outhit (`KismetSystemLibrary.CapsuleTraceSingle` :`Start` (`SceneComponent.K2_GetComponentLocation` (`self.Camera2`)) :`End` (`SceneComponent.K2_GetComponentLocation` (`Actor.RootComponent` (`Controller.K2_GetPawn` (`GameplayStatics.GetPlayerController` 0)))) :`Radius` 42.0 :`TraceChannel` "TraceTypeQuery1" :`DrawDebugType` "ForDuration"))
  (bind _asactor (cast `Actor` (`.HitActor` (`GameplayStatics.BreakHitResult` _outhit))))
  (`KismetSystemLibrary.PrintString` (`KismetSystemLibrary.GetDisplayName` _asactor)))

(fn `UserConstructionScript`)