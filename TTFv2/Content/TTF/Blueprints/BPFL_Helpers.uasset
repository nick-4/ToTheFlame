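; Blueprint function library of small gameplay helpers for noise, teams and health bars.
; MakeNoise reports a tagged AI noise event at a location and draws a brief debug sphere there.
; GetTeamName reads the team name from an actor's BP_TeamComponent, falling back to "None" if absent.
; SwitchPersonalHealthBar toggles the personal health bar on pawns that cast to BP_BaseChar.
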(fn `GetTeamName`
  (params (Actor :type "Actor Object Reference"))
  (returns (TeamName :type Name))
  (bind _returnvalue (`Actor.GetComponentByClass` Actor "/Game/TTF/Blueprints/Characters/Enemies/Components/BP_TeamComponent.BP_TeamComponent_C"))
  (`/Engine/EditorBlueprintResources/StandardMacros.IsValid` _returnvalue
    (:`Is Valid`
      (return (`/Game/TTF/Blueprints/Characters/Enemies/Components/BP_TeamComponent.TeamName` _returnvalue)))
    (:`Is Not Valid`
      (return "None"))))

(fn `MakeNoise`
  (params (NoiseLocation :type "Vector Structure") (Tag :type Name))
  (`AISense_Hearing.ReportNoiseEvent` null NoiseLocation 1.0 null 0.0 Tag)
  (`KismetSystemLibrary.DrawDebugSphere` null NoiseLocation 10.0 12 (struct :`R` 1.0 :`G` 0.803365 :`B` 0.100902 :`A` 1.0) 2.0))

(fn `SwitchPersonalHealthBar`
  (params (Pawn :type "Actor Object Reference") (ON :type Boolean))
  (bind _asbp_base_char (cast `/Game/TTF/Blueprints/Characters/BP_BaseChar` Pawn))
  (`/Game/TTF/Blueprints/Characters/BP_BaseChar.TurnPersonalHealthBarOn` _asbp_base_char ON))