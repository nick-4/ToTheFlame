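; Base character Blueprint with replicated health, an overhead-style personal health bar widget and ragdoll death.
; Construction sets the starting health, and ChangeHealth applies a delta clamped between zero and the maximum.
; OnRep_Health refreshes the bar, fires the OnHealthUpdated dispatcher and checks for death.
; At zero health Die runs once, disabling movement and capsule collision, simulating mesh physics and hiding the bar.
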(event `self.ReceiveBeginPlay`
  (`self.UpdateHealthBarMethod`))

(fn `ChangeHealth`
  (params (ChangeValue :type "Float (double-precision)"))
  (set `self.Health` (`KismetMathLibrary.FClamp` (+ ChangeValue (`self.Health`)) 0.0 (`self.MaxHealth`))))

(fn `Die`
  (set `self.IsDead?` true)
  (`self.RagdollOn`)
  (`self.TurnPersonalHealthBarOn` false))

(fn `OnRep_Health`
  (`self.UpdateHealthBarMethod`)
  (`self.OnHealthUpdated` (`self.Health`) (`self.MaxHealth`))
  (`self.TurnOnRagdollIfNeeded`))

(fn `TurnPersonalHealthBarOn`
  (params (bNewVisibility :type Boolean))
  (`SceneComponent.SetVisibility` (`self.HealthBarWidget`) bNewVisibility true))

(fn `UpdateHealthBarMethod`
  (bind _aswbp_personal_health_bar (cast `/Game/TTF/Blueprints/Widgets/WBP_PersonalHealthBar` (`WidgetComponent.GetUserWidgetObject` (`self.HealthBarWidget`))))
  (`ProgressBar.SetPercent` (`/Game/TTF/Blueprints/Widgets/WBP_PersonalHealthBar.HealthProgressBar` _aswbp_personal_health_bar) (/ (`self.Health`) (`self.MaxHealth`))))

(fn `UserConstructionScript`
  (`self.Initialize`))