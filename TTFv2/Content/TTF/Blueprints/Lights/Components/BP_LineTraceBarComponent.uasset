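; Scene component that finds light-vulnerable actors in front of a rectangular light area, using line traces.
; TraceForTargets derives corners and step sizes from width, height and world transform, then runs grid-based forward object traces over pawns and world objects.
; Hit actors implementing BPI_LightVulnerableV2 collect in TraceResults and are copied into the returned interface collection.
; Debug trace drawing and size printing remain active, and alternative trace methods are left disconnected.
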(fn `CalculateLayoutValues`
  (bind _returnvalue (`self.K2_GetComponentRotation`))
  (bind _width (`self.Width`))
  (bind _height (`self.Height`))
  (bind _returnvalue_2 (* (`self.Up`) (`self.Height`)))
  ;[1 1 1] Float Values
  (set `self.WStep` (/ _width (`KismetMathLibrary.Conv_IntToDouble` (`self.StepsWidth`))))
  (`KismetSystemLibrary.PrintText` (`|FormatText` "{w}, {h}" _width _height))
  (set `self.HStep` (/ _height (`KismetMathLibrary.Conv_IntToDouble` (`self.StepsHeight`))))
  (set `self.HalfHeight` (/ (`self.Height`) 2.0))
  (set `self.HalfWidth` (/ (`self.Width`) 2.0))
  ;[1 1 1] Vector Values
  (set `self.Position` (`self.K2_GetComponentLocation`))
  (set `self.Forward` (`KismetMathLibrary.GetForwardVector` _returnvalue))
  (set `self.Right` (`KismetMathLibrary.GetRightVector` _returnvalue))
  (set `self.Up` (`KismetMathLibrary.GetUpVector` _returnvalue))
  ;[1 1 1] Corners
  (bind _output_get (set `self.BottomLeft` (- (- (`self.Position`) (* (`self.Right`) (`self.HalfWidth`))) (* (`self.Up`) (`self.HalfHeight`)))))
  (set `self.TopLeft` (+ _output_get _returnvalue_2))
  (bind _output_get_2 (set `self.BottomRight` (+ _output_get (* (`self.Right`) (`self.Width`)))))
  (set `self.TopRight` (+ _returnvalue_2 _output_get_2)))

(fn `MakeATrace`
  (params (Start :type "Vector Structure") (End :type "Vector Structure"))
  ;[1 1 1] Current Line Trace Implementation
  (bind _outhit (`KismetSystemLibrary.LineTraceSingleForObjects` :`Start` Start :`End` End :`ObjectTypes` (`|MakeArray` "ObjectTypeQuery3" "ObjectTypeQuery1" "ObjectTypeQuery2" :!type "EObjectTypeQuery Enum") :`DrawDebugType` "ForOneFrame"))
  (cast `/Game/TTF/Blueprints/Lights/BPI_LightVulnerableV2` (`.HitActor` (`GameplayStatics.BreakHitResult` _outhit)))
  (`BlueprintSetLibrary.Set_Add` (`self.TraceResults`) (`.HitActor` (`GameplayStatics.BreakHitResult` _outhit))))

(fn `TraceForTargets`
  (returns (TracesVulnerableResults :type "Array of /Game/TTF/Blueprints/Lights/BPI_LightVulnerableV2 Interface"))
  (`|ExecutionSequence`
    (:`then_0`
      (`self.CalculateLayoutValues`))
    (:`then_1`
      (`self.TraceCycle`))
    (:`then_2`
      (`self.FillArrayOfVulnerables`))
    (:`then_3`
      (return (`self.TracesVulnerableResults`)))))