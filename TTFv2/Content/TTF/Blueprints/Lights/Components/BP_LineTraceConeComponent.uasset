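; Light component that finds light-vulnerable targets inside a cone by casting line traces from its world transform.
; TraceForTargets clears past results, derives the cone layout, then traces concentric rings plus a center ray.
; Ring count comes from outer radius over arc spacing on a unit circle, while every ring uses the same step count.
; Trace hits are cast to BPI_LightVulnerableV2 to build the returned target list.
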(fn `CalculateLayoutValues`
  (bind _returnvalue (`self.K2_GetComponentRotation`))
  ;[1 1 1] Vector Values
  (set `self.Position` (`self.K2_GetComponentLocation`))
  (set `self.Forward` (`KismetMathLibrary.GetForwardVector` _returnvalue))
  (set `self.Right` (`KismetMathLibrary.GetRightVector` _returnvalue))
  (set `self.Up` (`KismetMathLibrary.GetUpVector` _returnvalue))
  ;[1 1 1] 1cm Circle Properties
  (bind _output_get (set `self.OuterArcDegreese` (/ 360.0 (`KismetMathLibrary.Conv_IntToDouble` (`self.OuterCircleSteps`)))))
  (bind _output_get_2 (set `self.OuterCircleRadius` (`KismetMathLibrary.DegSin` (`self.HalfAngle`))))
  (set `self.OuterArcLen` (/ (* _output_get (`KismetMathLibrary.MultiplyByPi` _output_get_2)) 180.0))
  ;[1 1 1] RAngle Steps
  (bind _output_get_3 (set `self.SourceAngleStepsN` (`KismetMathLibrary.FCeil` (/ (`self.OuterCircleRadius`) (`self.OuterArcLen`)))))
  (set `self.SourceAngleStep` (/ (`self.HalfAngle`) (`KismetMathLibrary.Conv_IntToDouble` _output_get_3))))

(fn `GetConeRotator`
  (params (SourceHalfAngle :type "Float (double-precision)") (CircleAngle :type "Float (double-precision)"))
  (returns (ReturnValue :type "Rotator Structure"))
  (bind _returnvalue (`self.GetConeVector` SourceHalfAngle CircleAngle))
  (return (`KismetMathLibrary.MakeRotFromX` _returnvalue)))

(fn `GetConeVector`
  (params (SourceHalfAngle :type "Float (double-precision)") (CircleAngle :type "Float (double-precision)"))
  (returns (ReturnValue :type "Vector Structure"))
  (bind _returnvalue (`KismetMathLibrary.DegSin` SourceHalfAngle))
  (return (+ (* (`self.Forward`) (`KismetMathLibrary.DegCos` SourceHalfAngle)) (* (* (`self.Up`) (`KismetMathLibrary.DegSin` CircleAngle)) _returnvalue) (* (* (`self.Right`) (`KismetMathLibrary.DegCos` CircleAngle)) _returnvalue))))

(fn `TraceCircle`
  (params (SourceHalfAngle :type "Float (double-precision)") (StepsNumber :type Integer))
  (bind _position (`self.Position`))
  (for _index (range 1 (+ StepsNumber 1))
    (bind _returnvalue (`self.GetConeVector` SourceHalfAngle (* _index (/ 360.0 (`KismetMathLibrary.Conv_IntToDouble` StepsNumber)))))
    (`/Game/TTF/Blueprints/Lights/BPFL_LightHelpers.MakeALightTrace` _position (+ _position (* _returnvalue (`self.LightTraceDistance`))) (`self.TraceResults`))))

(fn `TraceForTargets`
  (returns (TracesVulnerableResults :type "Array of /Game/TTF/Blueprints/Lights/BPI_LightVulnerableV2 Interface"))
  (`|ExecutionSequence`
    (:`then_0`
      (`self.ClearTraceLists`))
    (:`then_1`
      (`self.CalculateLayoutValues`))
    (:`then_2`
      (`self.Trace Cycle`))
    (:`then_3`
      (`self.FillArrayOfVulnerables`))
    (:`then_4`
      (return (`self.TracesVulnerableResults`)))))