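; Spot light actor that pairs its visible cone with a line trace cone component for detecting targets within the light.
; The construction script sizes the SpotLight from LightConeParams, copies those params into BPLineTraceConeComponent and has it calculate its layout.
; It then rotates six debug arrows evenly around the cone edge using the component's cone rotator.
; TraceForTargets passes through to the component, and the event graph has no active logic.
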(fn `PositionDebugArrows`
  (locals (LocalArrows :type "Array of ArrowComponent Object Reference"))
  (bind _bp_linetraceconecomponent (`self.BP_LineTraceConeComponent`))
  (set `local.LocalArrows` (`|MakeArray` (`self.Arrow01`) (`self.Arrow02`) (`self.Arrow03`) (`self.Arrow04`) (`self.Arrow05`) (`self.Arrow06`)))
  (for _index (range 6)
    (bind _returnvalue (`/Game/TTF/Blueprints/Lights/Components/BP_LineTraceConeComponent.GetConeRotator` _bp_linetraceconecomponent (`/Game/TTF/Blueprints/Lights/Components/BP_LineTraceConeComponent.HalfAngle` _bp_linetraceconecomponent) (* _index 60.0)))
    (`SceneComponent.K2_SetWorldRotation` (`|GetArrayItem` (`local.LocalArrows`) _index) _returnvalue false false)))

(fn `TraceForTargets`
  (returns (Targets :type "Array of /Game/TTF/Blueprints/Lights/BPI_LightVulnerableV2 Interface"))
  (bind _tracesvulnerableresults (`/Game/TTF/Blueprints/Lights/Components/BP_LineTraceConeComponent.TraceForTargets` (`self.BP_LineTraceConeComponent`)))
  (return _tracesvulnerableresults))

(fn `UserConstructionScript`
  (bind _bp_linetraceconecomponent (`self.BP_LineTraceConeComponent`))
  (`parent.UserConstructionScript`)
  (`self.SetupSponLight`)
  (`/Game/TTF/Blueprints/Lights/BPFL_LightHelpers.CopyLightConeValuesToComponent` (`self.LightConeParams`) _bp_linetraceconecomponent)
  (`/Game/TTF/Blueprints/Lights/Components/BP_LineTraceConeComponent.CalculateLayoutValues` _bp_linetraceconecomponent)
  (`self.PositionDebugArrows`))