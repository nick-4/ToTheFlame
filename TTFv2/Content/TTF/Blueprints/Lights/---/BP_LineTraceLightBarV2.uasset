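; BP_LineTraceLightBarV2 is a light bar actor that pairs a rect light with a line trace component to trace for targets.
; Its construction script sizes the light from LightBarParams, copies those values to the component and has it calculate layout values.
; Four debug arrows are then moved to the component's computed corners.
; TraceForTargets delegates to the component and returns its result, and the event graph holds only disabled stubs.
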(fn `PositionDebugArrows`
  (bind _bp_linetracebarcomponent (`self.BP_LineTraceBarComponent`))
  (`|ExecutionSequence`
    (:`then_0`
      (`SceneComponent.K2_SetWorldLocation` (`self.BLArrow`) (`/Game/TTF/Blueprints/Lights/Components/BP_LineTraceBarComponent.BottomLeft` _bp_linetracebarcomponent) false true))
    (:`then_1`
      (`SceneComponent.K2_SetWorldLocation` (`self.BRArrow`) (`/Game/TTF/Blueprints/Lights/Components/BP_LineTraceBarComponent.BottomRight` _bp_linetracebarcomponent) false true))
    (:`then_2`
      (`SceneComponent.K2_SetWorldLocation` (`self.TLArrow`) (`/Game/TTF/Blueprints/Lights/Components/BP_LineTraceBarComponent.TopLeft` _bp_linetracebarcomponent) false true))
    (:`then_3`
      (`SceneComponent.K2_SetWorldLocation` (`self.TRArrow`) (`/Game/TTF/Blueprints/Lights/Components/BP_LineTraceBarComponent.TopRight` _bp_linetracebarcomponent) false false))))

(fn `TraceForTargets`
  (returns (Targets :type "Array of /Game/TTF/Blueprints/Lights/BPI_LightVulnerable Interface"))
  (locals (WStep :type "Float (double-precision)" :default 0.0) (HStep :type "Float (double-precision)" :default 0.0) (HalfHeight :type "Float (double-precision)" :default 0.0) (HalfWidth :type "Float (double-precision)" :default 0.0) (Position :type "Vector Structure" :default (0.0 0.0 0.0)) (Forward :type "Vector Structure" :default (0.0 0.0 0.0)) (Right :type "Vector Structure" :default (0.0 0.0 0.0)) (Up :type "Vector Structure" :default (0.0 0.0 0.0)) (BottomLeft :type "Vector Structure" :default (0.0 0.0 0.0)))
  (bind _tracesvulnerableresults (`/Game/TTF/Blueprints/Lights/Components/BP_LineTraceBarComponent.TraceForTargets` (`self.BP_LineTraceBarComponent`)))
  (return _tracesvulnerableresults))

(fn `UserConstructionScript`
  (bind _bp_linetracebarcomponent (`self.BP_LineTraceBarComponent`))
  (`parent.UserConstructionScript`)
  (`self.SetupRectLight`)
  (`/Game/TTF/Blueprints/Lights/BPFL_LightHelpers.CopyLightBarValuesToComponent` (`self.LightBarParams`) _bp_linetracebarcomponent)
  (`/Game/TTF/Blueprints/Lights/Components/BP_LineTraceBarComponent.CalculateLayoutValues` _bp_linetracebarcomponent)
  (`self.PositionDebugArrows`))