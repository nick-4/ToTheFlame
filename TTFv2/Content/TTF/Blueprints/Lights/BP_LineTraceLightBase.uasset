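; BP_LineTraceLightBase is a base Blueprint for lights that damage traced targets while switched on.
; Each tick while IsON is set, it passes the results of TraceForTargets and the frame delta to BPLightDamageComponent's DamageAll.
; TraceForTargets is an empty stub here, leaving the trace to child classes.
; TurnLightOn sets IsON, whose RepNotify broadcasts LightOnStateChanged.
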(event `self.ReceiveTick`
  (params (DeltaSeconds :type "Float (single-precision)"))
  (if (`self.IsON`)
    (bind _targets (`self.TraceForTargets`))
    (`/Game/TTF/Blueprints/Lights/Components/BP_LightDamageComponent.DamageAll` (`self.BP_LightDamageComponent`) DeltaSeconds _targets)))

(fn `OnRep_IsON`
  (`self.LightOnStateChanged` (`self.IsON`)))

(fn `TraceForTargets`
  (returns (Targets :type "Array of /Game/TTF/Blueprints/Lights/BPI_LightVulnerable Interface"))
  (return))

(fn `TurnLightOn`
  (params (`On?` :type Boolean))
  (set `self.IsON` `On?`))

(fn `UserConstructionScript`)