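; BP_LineTraceLightBar is a light actor that finds light-vulnerable actors inside a rectangular beam using parallel line traces.
; TraceForTargets builds a width-by-height grid centered on the actor, moves four debug arrows to its corners and traces forward from each point.
; MakeATrace runs object traces with debug drawing, keeping hits that implement BPI_LightVulnerableV2, which TraceForTargets returns as an interface array.
; Its event graph is inactive, so tracing runs only when called.
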(fn `MakeATrace`
  (params (Start :type "Vector Structure") (End :type "Vector Structure"))
  (bind _outhit (`KismetSystemLibrary.LineTraceSingleForObjects` :`Start` Start :`End` End :`ObjectTypes` (`|MakeArray` "ObjectTypeQuery3" "ObjectTypeQuery1" "ObjectTypeQuery2" :!type "EObjectTypeQuery Enum") :`DrawDebugType` "ForOneFrame"))
  (cast `/Game/TTF/Blueprints/Lights/BPI_LightVulnerableV2` (`.HitActor` (`GameplayStatics.BreakHitResult` _outhit)))
  (`BlueprintSetLibrary.Set_Add` (`self.TraceResults`) (`.HitActor` (`GameplayStatics.BreakHitResult` _outhit))))

(fn `TraceForTargets`
  (returns (Targets :type "Array of /Game/TTF/Blueprints/Lights/BPI_LightVulnerableV2 Interface"))
  (locals (WStep :type "Float (double-precision)" :default 0.0) (HStep :type "Float (double-precision)" :default 0.0) (HalfHeight :type "Float (double-precision)" :default 0.0) (HalfWidth :type "Float (double-precision)" :default 0.0) (Position :type "Vector Structure" :default (0.0 0.0 0.0)) (Forward :type "Vector Structure" :default (0.0 0.0 0.0)) (Right :type "Vector Structure" :default (0.0 0.0 0.0)) (Up :type "Vector Structure" :default (0.0 0.0 0.0)) (BottomLeft :type "Vector Structure" :default (0.0 0.0 0.0)))
  (bind _returnvalue (`self.K2_GetActorRotation`))
  (bind _halfheight (`local.HalfHeight`))
  (bind _halfwidth (`local.HalfWidth`))
  (bind _returnvalue_2 (* _halfheight -1.0))
  (bind _returnvalue_3 (* _halfwidth -1.0))
  (`|ExecutionSequence`
    (:`then_0`
      ;[1 1 1] Local Initialization
      (set `local.WStep` (/ (`self.Width`) (`KismetMathLibrary.Conv_IntToDouble` (`self.StepsWidth`))))
      (set `local.HStep` (/ (`self.Height`) (`KismetMathLibrary.Conv_IntToDouble` (`self.StepsHeight`))))
      (set `local.HalfHeight` (/ (`self.Height`) 2.0))
      (set `local.HalfWidth` (/ (`self.Width`) 2.0))
      (set `local.Position` (`self.K2_GetActorLocation`))
      (set `local.Forward` (`KismetMathLibrary.GetForwardVector` _returnvalue))
      (set `local.Right` (`KismetMathLibrary.GetRightVector` _returnvalue))
      (set `local.Up` (`KismetMathLibrary.GetUpVector` _returnvalue))
      (set `local.BottomLeft` (- (- (`local.Position`) (* (`local.Right`) (`local.HalfWidth`))) (* (`local.Up`) (`local.HalfHeight`)))))
    (:`then_1`
      ;[1 1 1] Move Debug Arrows
      (`SceneComponent.K2_SetRelativeLocation` (`self.BLArrow`) (`KismetMathLibrary.MakeVector` 0.0 _returnvalue_3 _returnvalue_2) false true)
      (`SceneComponent.K2_SetRelativeLocation` (`self.BRArrow`) (`KismetMathLibrary.MakeVector` 0.0 _halfwidth _returnvalue_2) false true)
      (`SceneComponent.K2_SetRelativeLocation` (`self.TLArrow`) (`KismetMathLibrary.MakeVector` 0.0 _returnvalue_3 _halfheight) false true)
      (`SceneComponent.K2_SetRelativeLocation` (`self.TRArrow`) (`KismetMathLibrary.MakeVector` 0.0 _halfwidth _halfheight) false true))
    (:`then_2`
      ;[1 1 1] Trace Cycle
      (for _index (range (+ (`self.StepsHeight`) 1))
        (for _index_2 (range (+ (`self.StepsWidth`) 1))
          (bind _returnvalue_4 (+ (* (`local.Up`) (* _index (`local.HStep`))) (* (`local.Right`) (* _index_2 (`local.WStep`))) (`local.BottomLeft`)))
          (`self.MakeATrace` _returnvalue_4 (+ _returnvalue_4 (* (`local.Forward`) (`self.LightTraceDistance`)))))))
    (:`then_3`
      ;[1 1 1] Create Array of Vulnerables
      (bind _result (`BlueprintSetLibrary.Set_ToArray` (`self.TraceResults`)))
      (for _array_element _result
        (bind _asbpi_light_vulnerable_v2 (cast `/Game/TTF/Blueprints/Lights/BPI_LightVulnerableV2` _array_element))
        (`KismetArrayLibrary.Array_Add` (`self.TraceResultsInterfaced`) _asbpi_light_vulnerable_v2)))
    (:`then_4`
      ;[1 1 1] Return Array
      (return (`self.TraceResultsInterfaced`)))))

(fn `UserConstructionScript`
  (`parent.UserConstructionScript`))