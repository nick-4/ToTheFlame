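; BP_Stone is a stone actor that damages characters and makes an AI-audible noise on impact.
; Hit and overlap events both feed HitAndDestroy, which ignores the stone's instigator.
; Any other contact reports a "Noise" event with the stone as instigator and spawns an explosion emitter; despite its name, MakeHitSound plays no audio.
; BP_BaseChar targets take melee damage, then the stone destroys itself regardless of target.
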(event `self.ReceiveHit`
  (params (MyComp :type "PrimitiveComponent Object Reference") (Other :type "Actor Object Reference") (OtherComp :type "PrimitiveComponent Object Reference") (bSelfMoved :type Boolean) (HitLocation :type "Vector Structure") (HitNormal :type "Vector Structure") (NormalImpulse :type "Vector Structure") (Hit :type "HitResult Structure (by ref)"))
  (`KismetSystemLibrary.PrintString` "!! Hit !!")
  (`self.HitAndDestroy` Other))

(event `self.ReceiveActorBeginOverlap`
  (params (OtherActor :type "Actor Object Reference"))
  (`self.HitAndDestroy` OtherActor))

(fn `DamageCharacter`
  (params (Character :type "/Game/TTF/Blueprints/Characters/BP_BaseChar Object Reference"))
  (`/Game/TTF/Blueprints/Characters/BP_BaseChar.ApplyMeleeDamage` Character (`self.Damage`)))

(fn `HitAndDestroy`
  (params (Object :type "Object Object Reference"))
  (if (not (== (`self.GetInstigator`) Object))
    (`self.MakeHitSound`)
    (`|ExecutionSequence`
      (:`then_0`
        (bind _asbp_base_char (cast `/Game/TTF/Blueprints/Characters/BP_BaseChar` Object))
        (`self.DamageCharacter` _asbp_base_char))
      (:`then_1`
        (`self.K2_DestroyActor`)))))

(fn `MakeHitSound`
  (bind _returnvalue (`self.K2_GetActorLocation`))
  (`AISense_Hearing.ReportNoiseEvent` _returnvalue 1.0 self 0.0 "Noise")
  (`GameplayStatics.SpawnEmitterAtLocation` "/Game/StarterContent/Particles/P_Explosion.P_Explosion" _returnvalue))

(fn `UserConstructionScript`)