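; BP_ActivateButton is an overlap-triggered button that switches a linked object on and off.
; When a BP_BaseChar begins overlapping, it calls Activate on ActorsToActivate through BPI_Activatable, and Deactivate when one stops overlapping.
; Damper position helpers look unfinished: neither is called from the event graph, the save graph does nothing, and the setter multiplies its input by zero.
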(event `self.ReceiveActorBeginOverlap`
  (params (OtherActor :type "Actor Object Reference"))
  (cast `/Game/TTF/Blueprints/Characters/BP_BaseChar` OtherActor)
  (bind _asbpi_activatable (cast `/Game/TTF/Blueprints/Objects/BPI_Activatable` (`self.ActorsToActivate`)))
  (`/Game/TTF/Blueprints/Objects/BPI_Activatable.Activate` _asbpi_activatable))

(event `self.ReceiveActorEndOverlap`
  (params (OtherActor :type "Actor Object Reference"))
  (cast `/Game/TTF/Blueprints/Characters/BP_BaseChar` OtherActor)
  (bind _asbpi_activatable (cast `/Game/TTF/Blueprints/Objects/BPI_Activatable` (`self.ActorsToActivate`)))
  (`/Game/TTF/Blueprints/Objects/BPI_Activatable.Deactivate` _asbpi_activatable))

(fn `UserConstructionScript`)